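; BP_Door is a level exit door that ends the game with a win screen when the player reaches it.
; Its Open event rotates the Scene component 90 degrees; the file does not show what calls it.
; It creates the YouWin widget at BeginPlay, and a box overlap by BP_ThirdPersonCharacter disables movement and input, then shows the widget and mouse cursor.
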(event `self.ReceiveBeginPlay`
  (bind _returnvalue (`|CreateWidget` "/Game/Corregir/Sector8/Widget_YouWin.Widget_YouWin_C"))
  (set `self.YouWin` _returnvalue))

(event `Open`
  (`SceneComponent.K2_SetRelativeRotation` (`self.Scene`) (struct :`Yaw` 90.0) false false))

(event `self.Box.OnComponentBeginOverlap`
  (params (OverlappedComponent :type "PrimitiveComponent Object Reference") (OtherActor :type "Actor Object Reference") (OtherComp :type "PrimitiveComponent Object Reference") (OtherBodyIndex :type Integer) (bFromSweep :type Boolean) (SweepResult :type "HitResult Structure (by ref)"))
  (bind _returnvalue (`GameplayStatics.GetPlayerController` 0))
  (bind _asbp_third_person_character (cast `/Game/Corregir/BP_ThirdPersonCharacter` OtherActor))
  (`CharacterMovementComponent.DisableMovement` (`Character.CharacterMovement` _asbp_third_person_character))
  (`self.DisableInput` _returnvalue null)
  (`UserWidget.AddToViewport` (`self.YouWin`) 0)
  (set `PlayerController.bShowMouseCursor` true _returnvalue))

(fn `UserConstructionScript`)