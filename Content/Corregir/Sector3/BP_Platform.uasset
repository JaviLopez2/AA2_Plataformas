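; BP_Platform is a moving platform that shuttles back and forth between two points.
; On BeginPlay it records the relative location of component R as the start and that of the Sphere component as the end.
; A Timeline lerps R between them, and a Forward flag on Finished alternates reversing and replaying it for an endless ping-pong loop.
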(event `self.ReceiveBeginPlay`
  (set `self.InitialPosition` (`SceneComponent.RelativeLocation` (`self.r`)))
  (set `self.FInalPosition` (`SceneComponent.RelativeLocation` (`self.Sphere`)))
  (`self.MovePlatform`))

(event `MovePlatform`
  (set `self.forward` true)
  (bind (_direction _alpha) (`Timeline|Timeline` :`NewTime` 1.0 :!via `PlayFromStart` :!label _label)
    (:`Update`
      (`SceneComponent.K2_SetRelativeLocation` (`self.r`) (`KismetMathLibrary.VLerp` (`self.InitialPosition`) (`self.FInalPosition`) _alpha) false false))
    (:`Finished`
      (if (`self.forward`)
        (`self.Reverse`)
        (else
          (`self.MovePlatform`))))))

(event `Reverse`
  (set `self.forward` false)
  (goto _label :!via `Reverse`))

(fn `UserConstructionScript`)