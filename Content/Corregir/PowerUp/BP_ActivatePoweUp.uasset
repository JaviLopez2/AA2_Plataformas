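; A pickup actor that grants the player either boots or a jetpack.
; When BP_ThirdPersonCharacter overlaps its sphere, the FirstPowerUp flag picks the upgrade, sets the matching flag on the character's GameManager and shows that gear on the manager's Character.
; The pickup then destroys itself.
; Its construction script applies a configurable static mesh to the visual component.
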(event `self.Sphere1.OnComponentBeginOverlap`
  (params (OverlappedComponent :type "PrimitiveComponent Object Reference") (OtherActor :type "Actor Object Reference") (OtherComp :type "PrimitiveComponent Object Reference") (OtherBodyIndex :type Integer) (bFromSweep :type Boolean) (SweepResult :type "HitResult Structure (by ref)"))
  (bind _asbp_third_person_character (cast `/Game/Corregir/BP_ThirdPersonCharacter` OtherActor))
  (if (`self.FirstPowerUp`)
    (bind _gamemanager (`/Game/Corregir/BP_ThirdPersonCharacter.GameManager` _asbp_third_person_character))
    (set `/Game/Corregir/BP_GameManager.hasBoots` true _gamemanager)
    (bind _character (`/Game/Corregir/BP_GameManager.Character` _gamemanager))
    (`/Game/Corregir/BP_ThirdPersonCharacter.ShowBoots` _character)
    (else
      (set `/Game/Corregir/BP_GameManager.hasJetpack` true _gamemanager)
      (`/Game/Corregir/BP_ThirdPersonCharacter.ShowJetpack` _character)))
  (`self.K2_DestroyActor`))

(fn `UserConstructionScript`
  (`StaticMeshComponent.SetStaticMesh` (`self.Sphere`) (`self.StaticMesh`)))