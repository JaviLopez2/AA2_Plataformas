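; BP_Jetpack is a jetpack whose battery color shows the third-person character's remaining fuel as green, yellow or red.
; BeginPlay finds the character and applies a dynamic material instance to the Jetpack mesh.
; Tick checks fuel bands, using DoOnce gates that reset one another so each band change fires once.
; A timeline then lerps the BatteryColor parameter from the current color to the new one.
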(event `self.ReceiveBeginPlay`
  (bind _returnvalue (`GameplayStatics.GetActorOfClass` "/Game/Corregir/BP_ThirdPersonCharacter.BP_ThirdPersonCharacter_C"))
  (set `self.Character` _returnvalue)
  (bind _returnvalue_2 (`KismetMaterialLibrary.CreateDynamicMaterialInstance` (`self.Material`)))
  (bind _output_get (set `self.NewVar` _returnvalue_2))
  (`PrimitiveComponent.SetMaterial` (`self.Jetpack`) 0 _output_get))

(event `CheckFuel`
  (bind _fuel (`/Game/Corregir/BP_ThirdPersonCharacter.Fuel` (`self.Character`)))
  (if (> _fuel 66.0)
    (`/Engine/EditorBlueprintResources/StandardMacros.DoOnce` false :!label _label
      (:`Completed`
        (`self.Reset2`)
        (`self.Reset3`)
        (set `self.NewColor` (`self.Green`))
        (`self.ChangeColor` :!label _label_2)))
    (elif (and (< _fuel 66.0) (> _fuel 33.0))
      (`/Engine/EditorBlueprintResources/StandardMacros.DoOnce` false :!label _label_3
        (:`Completed`
          (`self.Reset1`)
          (`self.Reset3`)
          (set `self.NewColor` (`self.Yellow`))
          (goto _label_2)))
      (elif (and (< _fuel 33.0) (> _fuel 0.0))
        (`/Engine/EditorBlueprintResources/StandardMacros.DoOnce` false :!label _label_4
          (:`Completed`
            (`self.Reset1`)
            (`self.Reset2`)
            (set `self.NewColor` (`self.Red`))
            (goto _label_2)))))))

(event `Reset1`
  (goto _label :!via `Reset`))

(event `Reset2`
  (goto _label_3 :!via `Reset`))

(event `Reset3`
  (goto _label_4 :!via `Reset`))

(event `ChangeColor`
  (bind _newcolor (`self.NewColor`))
  (bind (_direction _newtrack_0) (`Timeline|Timeline` :!via `PlayFromStart`)
    (:`Update`
      (`MaterialInstanceDynamic.SetVectorParameterValue` (`self.NewVar`) "BatteryColor" (`KismetMathLibrary.LinearColorLerp` (`self.CurrentColor`) _newcolor _newtrack_0)))
    (:`Finished`
      (set `self.CurrentColor` _newcolor))))

(event `self.ReceiveTick`
  (params (DeltaSeconds :type "Float (single-precision)"))
  (`self.CheckFuel`))

(fn `UserConstructionScript`)