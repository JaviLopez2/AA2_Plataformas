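; Game manager for a timed key puzzle that opens a door once at least two keys are collected before time runs out.
; Final starts a looping Countdown timer when one key is held; StopTimer gates its logic rather than clearing it.
; Success opens the Door with a sound, while timeout resets the count and time and re-shows every BP_Key.
; Key count and remaining time display through PrintString.
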(event `self.ReceiveBeginPlay`
  ;[0.1479 0.1009 1] Referencia al player y a las llaves.
  (bind _returnvalue (`GameplayStatics.GetActorOfClass` "/Game/ThirdPerson/Blueprints/BP_ThirdPersonCharacter.BP_ThirdPersonCharacter_C"))
  (set `self.Character` _returnvalue)
  (bind _outactors (`GameplayStatics.GetAllActorsOfClass` "/Game/BP_Key.BP_Key_C"))
  (set `self.Keys` _outactors))

(event `Countdown`
  ;[1 0 0.1203] Parar Contador
  (if (`self.stop timer`)
    _
    (elif (> (`self.TimeRemaining`) 0.0)
      ;[0.05404 1 0] Print Timer
      (`KismetSystemLibrary.PrintString` (`KismetStringLibrary.Conv_DoubleToString` (`self.TimeRemaining`)))
      ;[0 1 0.2366] Restar Tiempo
      (set `self.TimeRemaining` (- (`self.TimeRemaining`) (`self.timer`)))
      ;[1 0.679 0.3121] Si tengo las dos llaves se abre la puerta final.
      (if (>= (`self.keyNumber`) 2)
        (if (not (`self.Finish`))
          (set `self.Finish` true)
          (set `self.TimeRemaining` 0.0)))
      (elif (`self.Finish`)
        ;[0.4076 1 0] Puzzle Correcto
        (`KismetSystemLibrary.PrintString` "PuzzleCompletado")
        (set `self.stop timer` true)
        (`/Game/BP_Door.Open` (`self.Door`))
        (`GameplayStatics.PlaySound2D` "/Game/StarterContent/Audio/Explosion01.Explosion01" 1.0 1.0 0.0 null null)
        (else
          ;[1 0.302 0.312] Puzzle Incorrecto + Reiniciar puzzle
          (set `self.keyNumber` 0)
          (set `self.hasOneKey` false)
          (set `self.TimeRemaining` 5.0)
          (set `self.stop timer` true)
          (for _array_element (`self.Keys`)
            (`/Game/BP_Key.ShowKey` _array_element)))))))

(event `Final`
  ;[0.954 0.3524 1] Iniciar Timer
  (if (`self.hasOneKey`)
    (`KismetSystemLibrary.K2_SetTimer` null "Countdown" (`self.timer`) true)))

(event `self.ReceiveTick`
  (params (DeltaSeconds :type "Float (single-precision)"))
  ;[0 0.7108 1] Mostrar numero de llaves.
  (`KismetSystemLibrary.PrintString` (`KismetStringLibrary.Concat_StrStr` "Numero de llaves: " (`KismetStringLibrary.Conv_IntToString` (`self.keyNumber`))) true true (struct :`G` 0.66 :`B` 1.0 :`A` 1.0) 0.0))

(fn `UserConstructionScript`)