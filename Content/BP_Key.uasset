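; BP_Key is a collectible key that the third-person character picks up by overlapping its collision sphere.
; On pickup it updates key possession, key count and the timer flag on BP_GameManager, found at BeginPlay, then calls the manager's Final.
; The key is hidden rather than destroyed, with HideKey and ShowKey toggling mesh visibility and trigger collision so it can be restored.
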(event `self.ReceiveBeginPlay`
  (bind _returnvalue (`GameplayStatics.GetActorOfClass` "/Game/BP_GameManager.BP_GameManager_C"))
  (set `self.GameManager` _returnvalue))

(event `self.Sphere1.OnComponentBeginOverlap`
  (params (OverlappedComponent :type "PrimitiveComponent Object Reference") (OtherActor :type "Actor Object Reference") (OtherComp :type "PrimitiveComponent Object Reference") (OtherBodyIndex :type Integer) (bFromSweep :type Boolean) (SweepResult :type "HitResult Structure (by ref)"))
  (bind _gamemanager (`self.GameManager`))
  (cast `/Game/ThirdPerson/Blueprints/BP_ThirdPersonCharacter` OtherActor)
  (set `/Game/BP_GameManager.hasOneKey` true _gamemanager)
  (`/Engine/EditorBlueprintResources/StandardMacros.IncrementInt` (`/Game/BP_GameManager.keyNumber` _gamemanager)
    (:`  `
      (set `/Game/BP_GameManager.stop timer` false _gamemanager)
      (`/Game/BP_GameManager.Final` _gamemanager)
      (`self.HideKey`))))

(event `HideKey`
  ;[0.1823 0.1823 0.1823] Ocultar Llaves
  (`SceneComponent.SetVisibility` (`self.Sphere`) false true)
  (`PrimitiveComponent.SetCollisionEnabled` (`self.Sphere1`) "NoCollision"))

(event `ShowKey`
  ;[0.2776 0.6579 1] Mostrar Llaves
  (`SceneComponent.SetVisibility` (`self.Sphere`) true true)
  (`PrimitiveComponent.SetCollisionEnabled` (`self.Sphere1`) "QueryAndPhysics"))

(fn `UserConstructionScript`)